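; BP_SonarSource is a short-lived sonar pulse that registers with nearby visibility updaters and alerts monsters.
; On spawn, it sphere-traces at maximum radius, adds itself to each hit actor's SC_VisibilityUpdater and sends its location to any such actor that is a BP_Monster.
; It then destroys all other sonar sources, leaving one active.
; Tick eases Strength up over the initial duration, then ramps Decay until its lifespan ends.
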(event EventBeginPlay
  (Utilities|FlowControl|Sequence
    (:then_0
      (bind _outhits (Collision|MultiSphereTraceForObjects (Transformation|GetActorLocation) "0, 0, 0" (Variables|Stats|GetMaximumStrength) (Utilities|Array|MakeArray "ObjectTypeQuery1" "ObjectTypeQuery2" "ObjectTypeQuery3") false 0 "None"))
      (bind _array_element (Utilities|Array|ForEachLoopwithBreak _outhits)
        (:LoopBody
          (Utilities|IsValid (Actor|GetComponentbyClass (.HitActor (Collision|BreakHitResult _array_element)) "/Game/BluePrints/Components/SC_VisibilityUpdater.SC_VisibilityUpdater_C")
            (:Is%20Valid
              (Default|AddSonarSource (Actor|GetComponentbyClass (.HitActor (Collision|BreakHitResult _array_element)) "/Game/BluePrints/Components/SC_VisibilityUpdater.SC_VisibilityUpdater_C") self)
              (bind _asbp_monster (Utilities|Casting|CastToBP_Monster (.HitActor (Collision|BreakHitResult _array_element))))
              (Default|RecieveSonar _asbp_monster (Transformation|GetActorLocation)))))))
    (:then_1
      (Actor|SetLifeSpan (+ (Variables|Stats|GetSonarInititialDuration) (Variables|Stats|GetSonarDecayDuration))))
    (:then_2
      (CallFunction|KillOtherLights))))

(event Collision|EventActorBeginOverlap
  (params (OtherActor :type Actor%20Object%20Reference)))

(event EventTick
  (params (DeltaSeconds :type Float%20%28single-precision%29))
  (if (< (Actor|GetGameTimeSinceCreation) (Variables|Stats|GetSonarInititialDuration))
    (bind _output_get (Variables|DynamicVariables|SetStrength (Class|KismetMathLibrary|FInterpEaseinOut 0.0 (Variables|Stats|GetMaximumStrength) (/ (Actor|GetGameTimeSinceCreation) (Variables|Stats|GetSonarInititialDuration)) 3.0)))
    (else
      (Variables|DynamicVariables|SetDecay (Math|Float|Lerp 0.0 1.0 (Math|Float|Clamp(Float) (/ (- (Actor|GetGameTimeSinceCreation) (Variables|Stats|GetSonarInititialDuration)) (Variables|Stats|GetSonarDecayDuration))))))))

(fn ConstructionScript)

(fn KillOtherLights
  (bind _outactors (Actor|GetAllActorsOfClass "BP_SonarSource_C"))
  (for _array_element _outactors
    (if (!= _array_element self)
      (Actor|DestroyActor _array_element))))