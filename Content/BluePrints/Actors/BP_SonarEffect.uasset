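; BP_SonarEffect is a short-lived visual actor that renders an expanding sonar pulse.
; On BeginPlay it gives its static mesh a dynamic sonar material and plays a sonar sound at its location.
; Each Tick uses eased interpolation over its one-second lifetime to scale the mesh up massively while fading the material's opacity to zero, then the actor destroys itself.
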(event EventBeginPlay
  (bind _returnvalue (Rendering|Material|CreateDynamicMaterialInstance (Variables|Default|GetStaticMesh) 0 "/Game/Materials/Mat_Sonar_Effect_Inst_01.Mat_Sonar_Effect_Inst_01" :!class /Script/Engine.PrimitiveComponent))
  (Variables|Default|SetMat _returnvalue)
  (Audio|PlaySoundatLocation "/Game/Audio/audiofinal/sonarsound_Cue.sonarsound_Cue" (Transformation|GetWorldLocation (Variables|Default|GetDefaultSceneRoot))))

(event Collision|EventActorBeginOverlap
  (params (OtherActor :type Actor%20Object%20Reference)))

(event EventTick
  (params (DeltaSeconds :type Float%20%28single-precision%29))
  (bind _returnvalue (Actor|GetGameTimeSinceCreation))
  (bind _returnvalue_2 (/ _returnvalue 1.0))
  (bind _returnvalue_3 (Class|KismetMathLibrary|FInterpEaseinOut 0.0 1.5e+03 _returnvalue_2 3.0))
  (if (> (Actor|GetGameTimeSinceCreation) 1.0)
    (Actor|DestroyActor)
    (else
      (Transformation|SetWorldScale3D (Variables|Default|GetStaticMesh) (Math|Vector|MakeVector _returnvalue_3 _returnvalue_3 _returnvalue_3))
      (Rendering|Material|SetScalarParameterValue (Variables|Default|GetMat) "Opacity" (Class|KismetMathLibrary|FInterpEaseinOut 0.1 0.0 _returnvalue_2 3.0) :!class /Script/Engine.MaterialInstanceDynamic))))

(fn ConstructionScript)