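; Actor component that feeds sonar source data into its owner's static mesh materials, likely to drive sonar-based visibility.
; On BeginPlay it creates dynamic material instances for every mesh slot, takes the first BP_SonarSource found and pushes its location, strength and decay.
; AddSonarSource replaces that single source and enables LiveUpdate, which refreshes the parameters every Tick.
; AddMesh registers a mesh's materials for these updates.
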(event EventBeginPlay
  (bind _returnvalue (Components|GetOwner))
  (Utilities|FlowControl|Sequence
    (:then_0
      (bind _asprimitive_component (Utilities|Casting|CastToPrimitiveComponent (VehicleSound|GetRootComponent _returnvalue)))
      (Variables|Default|SetRoot _asprimitive_component))
    (:then_1
      (for _array_element (Actor|GetComponentsByClass _returnvalue "/Script/Engine.StaticMeshComponent")
        (CallFunction|AddMesh _array_element)))
    (:then_2
      (bind _outactors (Actor|GetAllActorsOfClass "/Game/BluePrints/Actors/BP_SonarSource.BP_SonarSource_C"))
      (Utilities|FlowControl|Sequence
        (:then_0
          (Variables|Default|SetSonarSource_1 (Utilities|Array|Get(acopy) _outactors)))))
    (:then_3
      (CallFunction|UpdateMaterialParams))))

(event EventTick
  (params (DeltaSeconds :type Float%20%28single-precision%29))
  (if (Variables|SonarStats|GetLiveUpdate)
    (CallFunction|UpdateMaterialParams)))

(fn UpdateMaterialParams
  (Utilities|IsValid (Variables|Default|GetSonarSource_1)
    (:Is%20Valid
      (for _array_element (Variables|Default|GetMats)
        (LocalVariables|SetCurrentMat _array_element)
        (Utilities|FlowControl|Sequence
          (:then_0
            ;[1 1 1] Source 1
            (Rendering|Material|SetVectorParameterValue (LocalVariables|GetCurrentMat) (Variables|Default|GetstrInputSourceLocation_1) (Math|Conversions|ToLinearColor(Vector) (Transformation|GetActorLocation (Variables|Default|GetSonarSource_1))) :!class /Script/Engine.MaterialInstanceDynamic))
          (:then_1
            (Rendering|Material|SetScalarParameterValue (LocalVariables|GetCurrentMat) (Variables|Default|GetstrInputSourceStrength_1) (Variables|/Game/BluePrints/Actors/BP_SonarSource.BP_SonarSource_C|GetStrength (Variables|Default|GetSonarSource_1)) :!class /Script/Engine.MaterialInstanceDynamic))
          (:then_2
            (Rendering|Material|SetScalarParameterValue (LocalVariables|GetCurrentMat) (Variables|Default|GetstrInputSourceDecay_1) (Variables|/Game/BluePrints/Actors/BP_SonarSource.BP_SonarSource_C|GetDecay (Variables|Default|GetSonarSource_1)) :!class /Script/Engine.MaterialInstanceDynamic)))))))

(fn AddMesh
  (params (NewMesh :type Mesh%20Component%20Object%20Reference))
  (bind _returnvalue (Rendering|Material|GetMaterials NewMesh))
  (for _index (range 0 (Utilities|Array|LastIndex _returnvalue))
    (bind _returnvalue_2 (Rendering|Material|CreateDynamicMaterialInstance NewMesh _index (Utilities|Array|Get(acopy) _returnvalue _index) :!class /Script/Engine.PrimitiveComponent))
    (Utilities|Array|Add (Variables|Default|GetMats) _returnvalue_2)))

(fn AddSonarSource
  (params (NewSource :type BP%20Sonar%20Source%20Object%20Reference))
  (Variables|Default|SetSonarSource_1 NewSource)
  (Variables|SonarStats|SetLiveUpdate true))