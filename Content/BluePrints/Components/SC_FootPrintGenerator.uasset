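; Component that leaves a trail of alternating left and right footprints behind its owning Character.
; Tick accumulates time while the character's movement velocity is non-zero and calls PlaceFootPrint whenever the step interval elapses.
; PlaceFootPrint offsets sideways by half the leg spacing, traces down against WorldStatic, and spawns an unrotated BP_FootPrint at the hit.
; The foot side flips only when the trace hits.
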(event EventBeginPlay
  (bind _ascharacter (Utilities|Casting|CastToCharacter (Components|GetOwner)))
  (Variables|Default|SetOwnerMovementComponent (Variables|/Script/Engine.Character|GetCharacterMovement _ascharacter)))

(event EventTick
  (params (DeltaSeconds :type Float%20%28single-precision%29))
  (if (> (Math|Vector|VectorLength (Variables|/Script/Engine.MovementComponent|GetVelocity (Variables|Default|GetOwnerMovementComponent))) 0.0)
    (Variables|RuntimeVars|SetTimeSinceFootStep (+ DeltaSeconds (Variables|RuntimeVars|GetTimeSinceFootStep)))
    (if (> (Variables|RuntimeVars|GetTimeSinceFootStep) (Variables|Stats|GetFootStepInterval))
      (CallFunction|PlaceFootPrint))))

(fn PlaceFootPrint
  (bind _returnvalue (Components|GetOwner))
  (bind _legsspacing (Variables|Default|GetlegsSpacing))
  (bind _returnvalue_2 (/ _legsspacing 2.0))
  (bind _returnvalue_3 (Transformation|GetActorLocation _returnvalue))
  (bind _returnvalue_4 (Transformation|GetActorRightVector _returnvalue))
  (bind _returnvalue_5 (* _returnvalue_4 _returnvalue_2))
  (if (Variables|RuntimeVars|GetLeftFoot)
    (LocalVariables|SetInitialLocation (+ _returnvalue_3 _returnvalue_5))
    (else
      (LocalVariables|SetInitialLocation (+ (* _returnvalue_5 -1.0) _returnvalue_3))))
  (Variables|RuntimeVars|SetTimeSinceFootStep 0.0)
  (bind (_outhit _returnvalue_6) (Collision|LineTraceForObjects (LocalVariables|GetInitialLocation) (+ (LocalVariables|GetInitialLocation) (* (Transformation|GetActorUpVector _returnvalue) -2e+03)) (Utilities|Array|MakeArray "ObjectTypeQuery1") false 0 "None"))
  (if _returnvalue_6
    (Game|SpawnActorfromClass "/Game/BluePrints/Actors/BP_FootPrint.BP_FootPrint_C" (Math|Transform|MakeTransform (.Location (Collision|BreakHitResult _outhit))) "Undefined" 0 0)
    (Variables|RuntimeVars|SetLeftFoot (not (Variables|RuntimeVars|GetLeftFoot)))))