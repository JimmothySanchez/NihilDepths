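; AI controller for the monster, which starts its behavior tree and seeds its blackboard.
; On BeginPlay it runs BT_Monster, then stores the first BP_WavePlayer found in the level as the player object and sets the level-of-alert key to an initial enum value.
; It has no per-frame logic of its own.
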(event EventBeginPlay
  (AI|RunBehaviorTree "/Game/BluePrints/Characters/Monster/BT_Monster.BT_Monster")
  (bind _outactors (Actor|GetAllActorsOfClass "/Game/BluePrints/Characters/BP_WavePLayer.BP_WavePlayer_C"))
  (AI|Components|Blackboard|SetValueasObject (AI|GetBlackboard self) (Variables|Default|GetPlayerVarName) (Utilities|Array|Get(acopy) _outactors))
  (AI|Components|Blackboard|SetValueasEnum (AI|GetBlackboard self) (Variables|Default|GetLevelOfAlertVarName) (Utilities|Enum|LiteralenumEnum_LevelOfAlert "NewEnumerator0")))

(event EventTick
  (params (DeltaSeconds :type Float%20%28single-precision%29)))

(fn ConstructionScript)