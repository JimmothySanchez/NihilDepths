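; BP_Monster is a monster character that reacts to sonar through RecieveSonar; its event graph is otherwise empty.
; A sonar hit writes the area of interest and a new alert level to the Blackboard, unless the enum check matches one specific level.
; That check reads the point-of-interest key as an enum, not the alert-state key.
; Every hit also spawns a BP_MonsterEcho at the capsule's transform.
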(event EventBeginPlay)

(event Collision|EventActorBeginOverlap
  (params (OtherActor :type Actor%20Object%20Reference)))

(event EventTick
  (params (DeltaSeconds :type Float%20%28single-precision%29)))

(fn ConstructionScript)

(fn RecieveSonar
  (params (AreaOfInterest :type Vector))
  (Utilities|FlowControl|Sequence
    (:then_0
      ;[1 1 1] Assign pont of interest
      (if (!= (Class|BlackboardComponent|GetValueasEnum (AI|GetBlackboard 0) (Variables|Default|GetPointOfInterestName)) (Utilities|Enum|LiteralenumEnum_LevelOfAlert "NewEnumerator2"))
        (AI|Components|Blackboard|SetValueasVector (AI|GetBlackboard 0) (Variables|Default|GetPointOfInterestName) AreaOfInterest)
        (AI|Components|Blackboard|SetValueasEnum (AI|GetBlackboard 0) (Variables|Default|GetAlertStateName) (Utilities|Enum|LiteralenumEnum_LevelOfAlert "NewEnumerator1"))))
    (:then_1
      (Game|SpawnActorfromClass "/Game/BluePrints/Actors/BP_MonsterEcho.BP_MonsterEcho_C" (Transformation|GetWorldTransform (Variables|Collision|GetCapsuleComponent)) "Undefined" 0 0))))