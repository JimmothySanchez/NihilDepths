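; BP_WavePLayer is the player character, with mouse look, yaw-relative movement, jumping and sonar abilities.
; Sonar spawns a source and effect at the camera, while the projectile variant launches from LaunchLocation; both require SonarCooldown to be expired, though nothing here sets it.
; KillThisDude pauses the game and shows the death screen with mouse-driven UI input.
; Debug-style keys take a high-res screenshot or quit.
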(event EventBeginPlay)

(event Collision|EventActorBeginOverlap
  (params (OtherActor :type Actor%20Object%20Reference)))

(event EventTick
  (params (DeltaSeconds :type Float%20%28single-precision%29)))

(event Input|ActionEvents|InputActionJump
  (params (Key :type Key%20Structure :default "AnyKey"))
  (:Pressed
    (Character|Jump)
    (Variables|/Script/Engine.CharacterMovementComponent|SetJumpZVelocity (Variables|Character|GetCharacterMovement) 365.0)))

(event Input|ActionEvents|InputActionSonarProjectile
  (params (Key :type Key%20Structure :default "AnyKey"))
  (:Pressed
    (if (<= (Variables|RuntimeVars|GetSonarCooldown) 0.0)
      (Game|SpawnActorfromClass "/Game/BluePrints/Actors/BP_Sonar_Projectile.BP_Sonar_Projectile_C" (Transformation|GetWorldTransform (Variables|Default|GetLaunchLocation)) "Undefined" 0 0))))

(event Input|ActionEvents|InputActionSonar
  (params (Key :type Key%20Structure :default "AnyKey"))
  (bind _camera (Variables|Default|GetCamera))
  (bind _returnvalue (Transformation|GetWorldTransform _camera))
  (:Pressed
    (if (<= (Variables|RuntimeVars|GetSonarCooldown) 0.0)
      (Game|SpawnActorfromClass "/Game/BluePrints/Actors/BP_SonarSource.BP_SonarSource_C" _returnvalue "AlwaysSpawn" 0 0)
      (Game|SpawnActorfromClass "/Game/BluePrints/Actors/BP_SonarEffect.BP_SonarEffect_C" _returnvalue "AlwaysSpawn" 0 0))))

(event Input|AxisEvents|InputAxisMoveForward
  (params (AxisValue :type Float%20%28single-precision%29))
  ;[1 1 1] Movement
  (Pawn|Input|AddMovementInput (Math|Vector|GetForwardVector (Math|Rotator|MakeRotator 0.0 0.0 (.Yaw (Math|Rotator|BreakRotator (Pawn|GetControlRotation :!class /Script/Engine.Pawn))))) AxisValue false))

(event Input|AxisEvents|InputAxisTurn
  (params (AxisValue :type Float%20%28single-precision%29))
  ;[1 1 1] Mouse Rotation
  (Pawn|Input|AddControllerYawInput AxisValue))

(event Input|AxisEvents|InputAxisLookUp
  (params (AxisValue :type Float%20%28single-precision%29))
  ;[1 1 1] Mouse Rotation
  (Pawn|Input|AddControllerPitchInput AxisValue))

(event Input|AxisEvents|InputAxisMoveRight
  (params (AxisValue :type Float%20%28single-precision%29))
  ;[1 1 1] Movement
  (Pawn|Input|AddMovementInput (Math|Vector|GetRightVector (Math|Rotator|MakeRotator 0.0 0.0 (.Yaw (Math|Rotator|BreakRotator (Pawn|GetControlRotation :!class /Script/Engine.Pawn))))) AxisValue false))

(event Input|KeyboardEvents|P
  (params (Key :type Key%20Structure :default "AnyKey"))
  (:Pressed
    (Development|ExecuteConsoleCommand "HighResShot 2")))

(event Input|KeyboardEvents|Escape
  (params (Key :type Key%20Structure :default "AnyKey"))
  (:Pressed
    (Game|QuitGame 0 "Quit")))

(fn ConstructionScript)

(fn KillThisDude
  (bind _returnvalue (Game|GetPlayerController 0))
  (Game|SetGamePaused true)
  (bind _returnvalue_2 (UserInterface|CreateWidget "/Game/UI/Widget_DeathScreen.Widget_DeathScreen_C"))
  (Variables|/Script/Engine.PlayerController|SetbEnableClickEvents _returnvalue true)
  (Variables|/Script/Engine.PlayerController|SetbShowMouseCursor _returnvalue true)
  (Input|SetInputModeUIOnly _returnvalue _returnvalue_2 "DoNotLock")
  (UserInterface|Viewport|AddtoPlayerScreen _returnvalue_2))